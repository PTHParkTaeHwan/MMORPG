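; BP_LobbyPC is the lobby player controller that sets up the lobby camera and menu UI.
; On BeginPlay, it blends the view to the first camera tagged MainCamera, then shows UI_LobbyWidget with UI-only input and a visible cursor.
; UI setup runs only if that camera is found.
; A JoinServer event opens the given IP address as a level to connect to a server.
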(event Custom|JoinServer
  (params (IpAddress :type String))
  (Game|OpenLevel(byName) (Utilities|String|StringToName IpAddress)))

(event EventBeginPlay
  (bind _self self)
  (bind _outactors (Actor|GetAllActorswithTag "MainCamera"))
  (if (> (Utilities|Array|Length _outactors) 0)
    (bind _ascamera_actor (Utilities|Casting|CastToCameraActor (Utilities|Array|Get(acopy) _outactors)))
    (Game|Player|SetViewTargetwithBlend _ascamera_actor 0.0 "VTBlend_Linear" 0.0 false)
    (bind _returnvalue (UserInterface|CreateWidget "/Game/Dev/Level/Lobby/UI_LobbyWidget.UI_LobbyWidget_C" _self))
    (bind _output_get (Variables|Default|SetUILobbyWidget _returnvalue))
    (Networking|SwitchHasAuthority
      (:Authority
        _)
      (:Remote
        _))
    (UserInterface|Viewport|AddtoViewport _output_get 0)
    (Input|SetInputModeUIOnly _self _output_get "DoNotLock")
    (Variables|Default|SetbShowMouseCursor _self true)))

(event EventTick
  (params (DeltaSeconds :type Float%20%28single-precision%29)))

(fn ConstructionScript)